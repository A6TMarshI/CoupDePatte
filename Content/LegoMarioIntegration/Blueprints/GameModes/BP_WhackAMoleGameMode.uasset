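; Game mode for the Whack-A-Mole game that configures a session from its level options string.
; It parses the options on BeginPlay and again whenever a level reload is requested through its delegate.
; Options fill random turn, last win, next spawn time and LevelPixelInfo's tower and trained-hand enums, with tower settings applied only as a complete set.
; Spawn time accepts comma decimals; Username is checked but unused.
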(event `self.ReceiveBeginPlay`
  (`self.ParseOptionString` (`self.OptionsString`))
  (add `self.OnRequestedReloadLevelDelegate` (delegate `OnRequestedReloadLevelDelegate_Event`))
  (`parent.ReceiveBeginPlay`))

(event `OnRequestedReloadLevelDelegate_Event` :!signature `self.OnRequestedReloadLevelDelegate`
  (params (OptionString :type String))
  (`self.ParseOptionString` OptionString))

(fn `ParseOptionString`
  (params (OptionString :type String))
  (bind (_levelpixelinfo_lvlpixeltag _levelpixelinfo_currentrow _levelpixelinfo_currentrowpixelcoordinate _levelpixelinfo_currentmoleremaining _levelpixelinfo_towermovement _levelpixelinfo_towerangle _levelpixelinfo_towerheight) (break `LevelPixelInfo` (`self.LevelPixelInfo`)))
  (bind (_levelpixelinfo_lvlpixeltag_2 _levelpixelinfo_currentrow_2 _levelpixelinfo_currentrowpixelcoordinate_2 _levelpixelinfo_currentmoleremaining_2 _levelpixelinfo_towermovement_2 _levelpixelinfo_towerangle_2 _levelpixelinfo_towerheight_2 _levelpixelinfo_handtrained) (break `LevelPixelInfo` (`self.LevelPixelInfo`)))
  (if (`GameplayStatics.HasOption` OptionString "RandomPlayerTurn")
    (switch `string` (`GameplayStatics.ParseOption` OptionString "RandomPlayerTurn")
      (:`Default`
        (set `self.bRandomPlayerTurn` false))
      (:`True`
        (set `self.bRandomPlayerTurn` true))))
  (if (and (`GameplayStatics.HasOption` OptionString "TowerHeight") (`GameplayStatics.HasOption` OptionString "TowerAngle") (`GameplayStatics.HasOption` OptionString "TowerMovement"))
    (set `self.LevelPixelInfo` (make `LevelPixelInfo` _levelpixelinfo_lvlpixeltag_2 _levelpixelinfo_currentrow_2 _levelpixelinfo_currentrowpixelcoordinate_2 _levelpixelinfo_currentmoleremaining_2 (cast `ETowerMovement` (`KismetMathLibrary.Conv_IntToByte` (`KismetStringLibrary.Conv_StringToInt` (`GameplayStatics.ParseOption` OptionString "TowerMovement")))) (cast `ETowerAngle` (`KismetMathLibrary.Conv_IntToByte` (`KismetStringLibrary.Conv_StringToInt` (`GameplayStatics.ParseOption` OptionString "TowerAngle")))) (cast `ETowerHeight` (`KismetMathLibrary.Conv_IntToByte` (`KismetStringLibrary.Conv_StringToInt` (`GameplayStatics.ParseOption` OptionString "TowerHeight")))) _levelpixelinfo_handtrained)))
  (if (`GameplayStatics.HasOption` OptionString "LastGameWin")
    (switch `string` (`GameplayStatics.ParseOption` OptionString "LastGameWin")
      (:`Default`
        (set `self.bLastGameWin` false))
      (:`True`
        (set `self.bLastGameWin` true))))
  (if (`GameplayStatics.HasOption` OptionString "HandTrained")
    (set `self.LevelPixelInfo` (make `LevelPixelInfo` _levelpixelinfo_lvlpixeltag _levelpixelinfo_currentrow _levelpixelinfo_currentrowpixelcoordinate _levelpixelinfo_currentmoleremaining _levelpixelinfo_towermovement _levelpixelinfo_towerangle _levelpixelinfo_towerheight (cast `EHandTrained` (`KismetMathLibrary.Conv_IntToByte` (`KismetStringLibrary.Conv_StringToInt` (`GameplayStatics.ParseOption` OptionString "HandTrained")))))))
  (if (`GameplayStatics.HasOption` OptionString "NextSpawnTime")
    (set `self.NextSpawnTime` (`KismetStringLibrary.Conv_StringToDouble` (`KismetStringLibrary.Replace` (`GameplayStatics.ParseOption` OptionString "NextSpawnTime") "," "."))))
  (if (`GameplayStatics.HasOption` OptionString "Username")
    _))

(fn `UserConstructionScript`)